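; GA_RangedAttack is an enemy gameplay ability that fires a projectile at the avatar's combat target.
; It turns the avatar to face the target and plays a randomly picked tagged attack montage.
; The montage's gameplay event triggers SpawnProjectile from the tagged socket toward the target, with optional pitch override.
; The ability ends shortly after the event or montage completion, or immediately on interruption or cancellation.
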(event `self.K2_ActivateAbility`
  (bind _returnvalue (`self.GetAvatarActorFromActorInfo`))
  (bind _returnvalue_2 (message `EnemyInterface.GetCombatTarget` _returnvalue))
  (bind _ascombat_interface (cast `CombatInterface` _returnvalue))
  (bind _returnvalue_3 (`Actor.K2_GetActorLocation` _returnvalue_2))
  (`CombatInterface.UpdateFacingTarget` _ascombat_interface _returnvalue_3)
  (bind _returnvalue_4 (message `CombatInterface.GetAttackMontages` (`self.GetAvatarActorFromActorInfo`)))
  (set `self.TaggedMontage` (`self.GetRandomTaggedMontageFromArray` _returnvalue_4))
  (`AbilityTask_PlayMontageAndWait.CreatePlayMontageAndWaitProxy` "None" (`.Montage` (break `TaggedMontage` (`self.TaggedMontage`))) 1.0 "None" false
    (:`then`
      (`AbilityTask_WaitGameplayEvent.WaitGameplayEvent` (`.MontageTag` (break `TaggedMontage` (`self.TaggedMontage`))) null true
        (:`EventReceived`
          (`self.SpawnProjectile` _returnvalue_3 (`.SocketTag` (break `TaggedMontage` (`self.TaggedMontage`))) (`self.Override Pitch`) (`self.Pitch Override`))
          (`KismetSystemLibrary.Delay` 0.5)
          (`self.K2_EndAbility`))))
    (:`OnCompleted`
      (`KismetSystemLibrary.Delay` 0.5)
      (`self.K2_EndAbility` :!label _label))
    (:`OnInterrupted`
      (goto _label))
    (:`OnCancelled`
      (goto _label))))